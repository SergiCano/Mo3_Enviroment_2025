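; Auto point light actor for a FluidNinjaLive foliage use case that brightens as the scene's directional light dims.
; On BeginPlay it grabs the first DirectionalLight and opens a gate for Tick updates.
; Each tick sets point light intensity to the capped, scaled reciprocal of the sun's intensity.
; Below a threshold, shadow casting moves from the directional light to the point light, which also gains its source radius.
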(event `self.ReceiveBeginPlay`
  (bind _light_component (`self.Light Component`))
  (bind _pointlight (`self.PointLight`))
  (bind _intensity (`LightComponentBase.Intensity` _light_component))
  (bind _returnvalue (< _intensity (`self.Point-To-Dir-LightThreshold`)))
  (bind _outactors (`GameplayStatics.GetAllActorsOfClass` "/Script/Engine.DirectionalLight"))
  (bind _lightcomponent (`Light.LightComponent` (`|GetArrayItem` _outactors)))
  (`/Engine/EditorBlueprintResources/StandardMacros.IsValid` _lightcomponent
    (:`Is Valid`
      (set `self.Light Component` _lightcomponent)
      (goto _label :!via `Open`))))

(event `self.ReceiveTick`
  (params (DeltaSeconds :type "Float (single-precision)"))
  (bind _light_component (`self.Light Component`))
  (bind _pointlight (`self.PointLight`))
  (bind _intensity (`LightComponentBase.Intensity` _light_component))
  (bind _returnvalue (< _intensity (`self.Point-To-Dir-LightThreshold`)))
  (`/Engine/EditorBlueprintResources/StandardMacros.Gate` true :!label _label
    (:`Exit`
      ;[0.1217 0.5041 1] Adjust PointLight intensity RECIPROCAL to Dir.Light intensity  ("automatically switches on in the dark")
      (`LightComponent.SetIntensity` _pointlight (* (`KismetMathLibrary.FMin` (/ 1.0 _intensity) (`self.MaxPointLightIntensity`)) (`self.LightMultiplier`)))
      ;[0.1217 0.5041 1] Switch OFF Directional Light Shadows, ON PointLight Shadows --- when Dir.Light intensity is LOW
      (`PointLightComponent.SetSourceRadius` _pointlight (* (`KismetMathLibrary.Conv_BoolToDouble` _returnvalue) (`self.LightSourceRadius`)))
      (`LightComponentBase.SetCastShadows` _pointlight _returnvalue)
      (`LightComponentBase.SetCastShadows` _light_component (not _returnvalue)))))

(fn `UserConstructionScript`)